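; Dungeon Master camera controller that moves, rotates and zooms the DungeonMasterCameraPawn from player input.
; Axis input and screen-edge mouse panning move the pawn in local space, with axis speed scaling by spring arm length.
; Holding Pan suspends navigation and opens gates that route mouse movement into roll and clamped pitch.
; Zoom steps the spring arm length within limits, and separate inputs reset pitch and zoom.
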(event EventBeginPlay
  (Utilities|FlowControl|Sequence
    (:then_0
      (Utilities|ReferenceCasts))))

(event Input|ActionEvents|InputActionPan
  (params (Key :type Key%20Structure :default "None"))
  (bind _camerapawnref (Variables|Default|GetCameraPawnRef))
  (bind _returnvalue (Transformation|GetActorRotation _camerapawnref))
  (bind (_roll _pitch _yaw) (Math|Rotator|BreakRotator _returnvalue))
  ;[1 1 1] Pan Y
  (:Pressed
    (Variables|Default|SetDisableCamNav true)
    (Utilities|FlowControl|Gate true) ; enters at Open
  )
  (:Released
    (Variables|Default|SetDisableCamNav false)
    (Utilities|FlowControl|Gate true) ; enters at Close
  ))

(event Input|ActionEvents|InputActionPan
  (params (Key :type Key%20Structure :default "None"))
  (bind _camerapawnref (Variables|Default|GetCameraPawnRef))
  (bind _returnvalue (Transformation|GetActorRotation _camerapawnref))
  (bind (_roll _pitch _yaw) (Math|Rotator|BreakRotator _returnvalue))
  ;[1 1 1] Pan X
  (:Pressed
    (Variables|Default|SetDisableCamNav true)
    (Utilities|FlowControl|Gate true) ; enters at Open
  )
  (:Released
    (Variables|Default|SetDisableCamNav false)
    (Utilities|FlowControl|Gate true) ; enters at Close
  ))

(event Input|ActionEvents|InputActionPanReset
  (params (Key :type Key%20Structure :default "None"))
  (bind _camerapawnref (Variables|Default|GetCameraPawnRef))
  (bind _returnvalue (Transformation|GetActorRotation _camerapawnref))
  (bind (_roll _pitch _yaw) (Math|Rotator|BreakRotator _returnvalue))
  ;[1 1 1] Pan Reset
  (:Pressed
    (Transformation|SetActorRotation _camerapawnref (Math|Rotator|MakeRotator _roll 0.0 _yaw))))

(event Input|ActionEvents|InputActionZoomIn
  (params (Key :type Key%20Structure :default "None"))
  (bind _camerapawnref (Variables|Default|GetCameraPawnRef))
  (bind _springarm (Variables|/Game/DungeonMaster/Blueprints/DungeonMasterCameraPawn.DungeonMasterCameraPawn_C|GetSpringArm _camerapawnref))
  ;[1 1 1] Camera Zoom controls
  (:Pressed
    (Variables|/Script/Engine.SpringArmComponent|SetTargetArmLength _springarm (Math|Float|Clamp(Float) (- (Variables|/Script/Engine.SpringArmComponent|GetTargetArmLength _springarm) (Variables|Default|GetZoomSensitivity)) 5e+02 (Variables|Default|GetMaxArmDistance)))))

(event Input|ActionEvents|InputActionZoomOut
  (params (Key :type Key%20Structure :default "None"))
  (bind _camerapawnref (Variables|Default|GetCameraPawnRef))
  (bind _springarm (Variables|/Game/DungeonMaster/Blueprints/DungeonMasterCameraPawn.DungeonMasterCameraPawn_C|GetSpringArm _camerapawnref))
  ;[1 1 1] Camera Zoom controls
  (:Pressed
    (Variables|/Script/Engine.SpringArmComponent|SetTargetArmLength _springarm (Math|Float|Clamp(Float) (+ (Variables|/Script/Engine.SpringArmComponent|GetTargetArmLength _springarm) (Variables|Default|GetZoomSensitivity)) 5e+02 (Variables|Default|GetMaxArmDistance)))))

(event Input|ActionEvents|InputActionZoomReset
  (params (Key :type Key%20Structure :default "None"))
  ;[1 1 1] Zoom Reset
  (:Pressed
    (Variables|/Script/Engine.SpringArmComponent|SetTargetArmLength (Variables|/Game/DungeonMaster/Blueprints/DungeonMasterCameraPawn.DungeonMasterCameraPawn_C|GetSpringArm (Variables|Default|GetCameraPawnRef)) 1.5e+03)))

(event Input|AxisEvents|InputAxisMoveForward
  (params (AxisValue :type Float%20%28single-precision%29))
  (bind _camerapawnref (Variables|Default|GetCameraPawnRef))
  ;[1 1 1] MovementX
  (if (not (Variables|Default|GetDisableCamNav))
    (Transformation|SetActorTransform _camerapawnref (Utilities|MovementX (CallFunction|MovementSpeedCalc) (Variables|Default|GetFastMoveMultiplier) AxisValue _camerapawnref))))

(event Input|AxisEvents|InputAxisMoveRight
  (params (AxisValue :type Float%20%28single-precision%29))
  (bind _movesensitivity (CallFunction|MovementSpeedCalc))
  (bind _fastmovemultiplier (Variables|Default|GetFastMoveMultiplier))
  (bind _camerapawnref (Variables|Default|GetCameraPawnRef))
  (bind _transform (Utilities|MovementY AxisValue _movesensitivity _fastmovemultiplier _camerapawnref))
  (bind (_location _rotation _scale) (Math|Transform|BreakTransform _transform))
  (bind (_x _y) (Math|Vector|BreakVector _location))
  ;[1 1 1] Movement Y
  (if (not (Variables|Default|GetDisableCamNav))
    (Transformation|SetActorTransform _camerapawnref (Math|Transform|MakeTransform (Math|Vector|MakeVector _x _y 1e+02) _rotation _scale))))

(event Input|MouseEvents|MouseX
  (params (AxisValue :type Float%20%28single-precision%29))
  (bind _camerapawnref (Variables|Default|GetCameraPawnRef))
  (bind _returnvalue (Transformation|GetActorRotation _camerapawnref))
  (bind (_roll _pitch _yaw) (Math|Rotator|BreakRotator _returnvalue))
  ;[1 1 1] Pan X
  (Utilities|FlowControl|Gate true
    (:Exit
      (Transformation|SetActorRotation _camerapawnref (Math|Rotator|MakeRotator (+ _roll (* (Variables|Default|GetPanSensitivity) AxisValue)) _pitch _yaw)))))

(event Input|MouseEvents|MouseY
  (params (AxisValue :type Float%20%28single-precision%29))
  (bind _camerapawnref (Variables|Default|GetCameraPawnRef))
  (bind _returnvalue (Transformation|GetActorRotation _camerapawnref))
  (bind (_roll _pitch _yaw) (Math|Rotator|BreakRotator _returnvalue))
  ;[1 1 1] Pan Y
  (Utilities|FlowControl|Gate true
    (:Exit
      (Transformation|SetActorRotation _camerapawnref (Math|Rotator|MakeRotator _roll (Math|Float|Clamp(Float) (+ _pitch (* (Variables|Default|GetPanSensitivity) AxisValue)) -15.0 45.0) _yaw)))))

(event Input|MouseEvents|MouseX
  (params (AxisValue :type Float%20%28single-precision%29))
  ;[1 1 1] Mouse Edge Panning
  (if (not (Variables|Default|GetDisableCamNav))
    (bind (_deltaxspeed _deltayspeed) (Utilities|ScreenEdgeMovement))
    (Transformation|AddActorLocalOffset (Variables|Default|GetCameraPawnRef) (Math|Vector|MakeVector _deltaxspeed _deltayspeed 0.0) true false)))

(event Input|MouseEvents|MouseY
  (params (AxisValue :type Float%20%28single-precision%29))
  ;[1 1 1] Mouse Edge Panning
  (if (not (Variables|Default|GetDisableCamNav))
    (Utilities|ScreenEdgeMovement) ; enters at Mouse Y
  ))

(fn ConstructionScript)

(fn MovementSpeedCalc
  (return (Math|Float|Clamp(Float) (/ (Variables|/Script/Engine.SpringArmComponent|GetTargetArmLength (Variables|/Game/DungeonMaster/Blueprints/DungeonMasterCameraPawn.DungeonMasterCameraPawn_C|GetSpringArm (Variables|Default|GetCameraPawnRef))) 1e+02) 5.0 2e+01)))