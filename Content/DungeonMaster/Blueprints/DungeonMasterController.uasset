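; Player controller for the Dungeon Master that handles forward/back navigation of the camera pawn.
; On BeginPlay it caches the player's DungeonMasterCameraPawn, and MoveForward input moves that pawn unless DisableCamNav is set.
; Speed derives from the clamped spring arm length, so it scales with zoom, and is passed with FastMoveMultiplier to MovementX.
; MovementX's local-X offset transform math appears unconnected to any output.
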(event EventBeginPlay
  (Utilities|FlowControl|Sequence
    (:then_0
      (Utilities|ReferenceCasts))))

(event Input|AxisEvents|InputAxisMoveForward
  (params (AxisValue :type Float%20%28single-precision%29))
  (bind _camerapawnref (Variables|Default|GetCameraPawnRef))
  (if (not (Variables|Default|GetDisableCamNav))
    (Transformation|SetActorTransform _camerapawnref (Utilities|MovementX (CallFunction|MovementSpeedCalc) (Variables|Default|GetFastMoveMultiplier) AxisValue _camerapawnref))))

(fn ConstructionScript)

(fn MovementSpeedCalc
  (return (Math|Float|Clamp(Float) (/ (Variables|/Script/Engine.SpringArmComponent|GetTargetArmLength (Variables|/Game/DungeonMaster/Blueprints/DungeonMasterCameraPawn.DungeonMasterCameraPawn_C|GetSpringArm (Variables|Default|GetCameraPawnRef))) 1e+02) 5.0 2e+01)))